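; MainLightChange is a rect light Blueprint that fades its light color to a requested color over a given transition time.
; The changeColor event stores the current and target colors, then restarts a Timeline with its play rate set to the inverse of that time.
; Each Timeline update lerps between the two colors and applies the result to the RectLightComponent.
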(event `changeColor`
  (params (NewColor :type "LinearColor Structure") (TransitionTimr :type "Float (double-precision)" :default 2.0))
  (set `self.New Color` NewColor)
  (set `self.CurrentColor` (`LightComponentBase.GetLightColor` (`self.RectLightComponent`)))
  (`TimelineComponent.SetPlayRate` (`self.Timeline`) (/ 1.0 TransitionTimr))
  (bind (_direction _newtrack_0) (`Timeline|Timeline` :!via `PlayFromStart`)
    (:`Update`
      (`LightComponent.SetLightColor` (`self.RectLightComponent`) (`KismetMathLibrary.LinearColorLerp` (`self.CurrentColor`) (`self.New Color`) _newtrack_0) true))))

(fn `UserConstructionScript`)